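; AmmoPickup_Base is a base ammo pickup actor that the player can interact with while in range.
; Overlapping its PickCollision binds the AmmoPickup event to the PlayerCharacter's interact input and shows the player's weapon pickup HUD.
; Ending the overlap unbinds the event and removes the HUD.
; The AmmoPickup event currently only prints the weapon class name and ammo count, without granting ammo.
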(event OnComponentBeginOverlap(PickCollision)
  (params (OverlappedComponent :type Primitive%20Component%20Object%20Reference) (OtherActor :type Actor%20Object%20Reference) (OtherComp :type Primitive%20Component%20Object%20Reference) (OtherBodyIndex :type Integer) (bFromSweep :type Boolean) (SweepResult :type Hit%20Result%20Structure%20%28by%20ref%29))
  (bind _asplayer_character (Utilities|Casting|CastToPlayerCharacter OtherActor))
  (EventDispatchers|BindEventtoInteract _asplayer_character (delegate Custom|AmmoPickup))
  (if (not (UserInterface|Viewport|IsinViewport (Variables|/Game/AdvancedLocomotionV4/Blueprints/CharacterLogic/PlayerCharacter.PlayerCharacter_C|GetWeaponPickHUD_ref _asplayer_character)))
    (UserInterface|Viewport|AddtoViewport (Variables|/Game/AdvancedLocomotionV4/Blueprints/CharacterLogic/PlayerCharacter.PlayerCharacter_C|GetWeaponPickHUD_ref _asplayer_character) 0)))

(event OnComponentEndOverlap(PickCollision)
  (params (OverlappedComponent :type Primitive%20Component%20Object%20Reference) (OtherActor :type Actor%20Object%20Reference) (OtherComp :type Primitive%20Component%20Object%20Reference) (OtherBodyIndex :type Integer))
  (bind _asplayer_character (Utilities|Casting|CastToPlayerCharacter OtherActor))
  (EventDispatchers|UnbindEventfromInteract _asplayer_character (delegate Custom|AmmoPickup))
  (Widget|RemovefromParent (Variables|/Game/AdvancedLocomotionV4/Blueprints/CharacterLogic/PlayerCharacter.PlayerCharacter_C|GetWeaponPickHUD_ref _asplayer_character)))

(event Custom|AmmoPickup
  (Development|PrintString (Utilities|GetClassDisplayName (Variables|Default|GetWeapon)))
  (Development|PrintString (Utilities|String|ToString(Integer) (Variables|Default|GetAmmoCount))))

(event EventBeginPlay
  (bind _asplayer_character (Utilities|Casting|CastToPlayerCharacter (Game|Player|GetPlayerPawn 0)))
  (Variables|Default|SetPlayerRef _asplayer_character))

(fn ConstructionScript)